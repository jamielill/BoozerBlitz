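; Melee customer NPC that, while angry and aware of the player, chases them to get within attack range.
; AI perception updates toggle the seeing flag for the first-person player character.
; Each tick it either re-issues an AI move to the player, flagging that it can attack on success, or, with the player unseen, stops and smoothly keeps turning toward its right to scan.
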(event OnTargetPerceptionUpdated(AIPerception)
  (params (Actor :type Actor%20Object%20Reference) (Stimulus :type AI%20Stimulus%20Structure))
  (Utilities|Casting|CastToBP_FirstPersonCharacter Actor)
  (if (.bsuccessfullysensed Stimulus)
    (Variables|Default|SetisSeeingPlayer true)
    (else
      (Variables|Default|SetisSeeingPlayer false))))

(event Custom|ChasePlayer
  (AI|AIMoveTo self "0, 0, 0" (Game|GetPlayerCharacter 0) 8e+01 false
    (:OnSuccess
      (Variables|Default|SetcanAttack true))))

(event EventTick
  (params (DeltaSeconds :type Float%20%28single-precision%29))
  (bind _returnvalue (Transformation|GetActorRotation))
  (if (Variables|Default|GetisSeeingPlayer)
    (if (Variables|Default|GetisAngry)
      (CallFunction|ChasePlayer))
    (else
      (Components|Movement|StopMovementImmediately (Variables|Character|GetCharacterMovement))
      (Transformation|SetActorRotation (Math|Interpolation|RInterpTo _returnvalue (Math|Conversions|RotationFromXVector (Math|Vector|RotateVector "0.000000,90.000000,0.000000" _returnvalue)) 0.0 5.0)))))

(fn ConstructionScript)