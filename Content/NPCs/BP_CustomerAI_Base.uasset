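; Base customer NPC AI that walks through the bar's door and heads for the queue.
; On BeginPlay it moves to the nearer BP_Doors point, waits, then crosses to the other, setting IsInside by direction.
; While inside, Tick reissues a move to the first BP_Bar queue spot.
; AI perception tracks player visibility, but the logic to chase when angry or otherwise stop and turn is disconnected.
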(event OnTargetPerceptionUpdated(AIPerception)
  (params (Actor :type Actor%20Object%20Reference) (Stimulus :type AI%20Stimulus%20Structure))
  (Utilities|Casting|CastToBP_FirstPersonCharacter Actor)
  (if (.bsuccessfullysensed Stimulus)
    (Variables|Default|SetisSeeingPlayer true)
    (else
      (Variables|Default|SetisSeeingPlayer false))))

(event Custom|ChasePlayer
  (AI|AIMoveTo self "0, 0, 0" (Game|GetPlayerCharacter 0) 8e+01 false
    (:OnSuccess
      (Variables|Default|SetcanAttack true))))

(event Custom|UseDoor
  (bind _returnvalue (Transformation|GetActorLocation))
  ;[1 1 1] finds the closest place to open the door from and moves to it
  (bind _returnvalue_2 (Actor|GetActorOfClass "/Game/Blueprints/BP_Doors.BP_Doors_C"))
  (if (< (Math|Vector|VectorLength (- (Transformation|GetWorldLocation (Variables|/Game/Blueprints/BP_Doors.BP_Doors_C|GetEnterRef _returnvalue_2)) _returnvalue)) (Math|Vector|VectorLength (- (Transformation|GetWorldLocation (Variables|/Game/Blueprints/BP_Doors.BP_Doors_C|GetExitRef _returnvalue_2)) _returnvalue)))
    (AI|AIMoveTo self (Transformation|GetWorldLocation (Variables|/Game/Blueprints/BP_Doors.BP_Doors_C|GetEnterRef _returnvalue_2)) 0 1.0 false
      (:OnSuccess
        ;[1 1 1] Walks through the door
        (Utilities|FlowControl|Delay 3.0)
        (AI|AIMoveTo self (Transformation|GetWorldLocation (Variables|/Game/Blueprints/BP_Doors.BP_Doors_C|GetExitRef _returnvalue_2)) 0 1.0 false
          (:OnSuccess
            (Variables|Default|SetisInside true)))))
    (else
      (AI|AIMoveTo self (Transformation|GetWorldLocation (Variables|/Game/Blueprints/BP_Doors.BP_Doors_C|GetExitRef _returnvalue_2)) 0 1.0 false
        (:OnSuccess
          (Utilities|FlowControl|Delay 3.0)
          (AI|AIMoveTo self (Transformation|GetWorldLocation (Variables|/Game/Blueprints/BP_Doors.BP_Doors_C|GetEnterRef _returnvalue_2)) 0 1.0 false
            (:OnSuccess
              (Variables|Default|SetisInside false))))))))

(event Custom|Queue
  (bind _returnvalue (Actor|GetActorOfClass "/Game/Blueprints/BP_Bar.BP_Bar_C"))
  (AI|AIMoveTo self (Transformation|GetWorldLocation (Variables|/Game/Blueprints/BP_Bar.BP_Bar_C|GetQueuePlace0Ref _returnvalue)) 0 5.0 false))

(event EventBeginPlay
  (CallFunction|UseDoor))

(event EventTick
  (params (DeltaSeconds :type Float%20%28single-precision%29))
  (if (Variables|Default|GetisInside)
    (CallFunction|Queue)))

(fn ConstructionScript)