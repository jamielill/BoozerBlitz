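; BP_Tap is an interactable tap that turns a pint glass's drink into water.
; A BP_PintGlass entering its Box is cached, shows the prompt widget and sets the player's CanInteract flag; any end overlap reverses the widget and flag.
; Interact reads the Water row from DT_DrinkData, writes its DrinkName to the cached glass, clears CanInteract and plays the pour sound at world origin.
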(event OnComponentBeginOverlap(Box)
  (params (OverlappedComponent :type Primitive%20Component%20Object%20Reference) (OtherActor :type Actor%20Object%20Reference) (OtherComp :type Primitive%20Component%20Object%20Reference) (OtherBodyIndex :type Integer) (bFromSweep :type Boolean) (SweepResult :type Hit%20Result%20Structure%20%28by%20ref%29))
  (bind _asbp_pint_glass (Utilities|Casting|CastToBP_PintGlass OtherActor))
  (Rendering|SetVisibility (Variables|Default|GetWidget) true false)
  (Variables|/Game/Blueprints/Player/FirstPerson/BP_FirstPersonCharacter.BP_FirstPersonCharacter_C|SetcanInteract (Variables|Default|GetPlayer) true))

(event OnComponentEndOverlap(Box)
  (params (OverlappedComponent :type Primitive%20Component%20Object%20Reference) (OtherActor :type Actor%20Object%20Reference) (OtherComp :type Primitive%20Component%20Object%20Reference) (OtherBodyIndex :type Integer))
  (Rendering|SetVisibility (Variables|Default|GetWidget) false false)
  (Variables|/Game/Blueprints/Player/FirstPerson/BP_FirstPersonCharacter.BP_FirstPersonCharacter_C|SetcanInteract (Variables|Default|GetPlayer) false))

(event EventBeginPlay
  (bind _returnvalue (Actor|GetActorOfClass "/Game/Blueprints/Player/FirstPerson/BP_FirstPersonCharacter.BP_FirstPersonCharacter_C"))
  (Variables|Default|SetPlayer _returnvalue))

(event EventInteract
  (bind _returnvalue (Utilities|GetDataTableRow "/Game/Blueprints/Drinks/DT_DrinkData.DT_DrinkData" "Water")
    (:then
      (Variables|/Game/Blueprints/Drinks/BP_Drink.BP_Drink_C|SetdrinkName (stale OnComponentBeginOverlap(Box) _asbp_pint_glass) (Utilities|String|StringToName (.drinkname _returnvalue)))
      (Variables|/Game/Blueprints/Player/FirstPerson/BP_FirstPersonCharacter.BP_FirstPersonCharacter_C|SetcanInteract (Variables|Default|GetPlayer) false)
      (Audio|SpawnSoundatLocation "/Game/Audio/SFX_Drink_Pour.SFX_Drink_Pour" "0, 0, 0" "0, 0, 0" 1.0 1.0 0.0 0 0))))

(fn ConstructionScript)