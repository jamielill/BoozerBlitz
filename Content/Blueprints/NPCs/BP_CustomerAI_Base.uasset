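; Base pub customer AI that walks in through the door, queues at the bar and orders a random drink from DT_DrinkData.
; A patience timer lowers its happiness score and turns it angry on expiry.
; Interacting with an overlapping drink pays the player by match (exact or same type) plus happiness, then the customer leaves and despawns.
; A wrong type also angers it, making it chase the player and deal damage on contact.
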(event OnComponentBeginOverlap(RecieveDrinkCollision)
  (params (OverlappedComponent :type Primitive%20Component%20Object%20Reference) (OtherActor :type Actor%20Object%20Reference) (OtherComp :type Primitive%20Component%20Object%20Reference) (OtherBodyIndex :type Integer) (bFromSweep :type Boolean) (SweepResult :type Hit%20Result%20Structure%20%28by%20ref%29))
  (bind _asbp_drink (Utilities|Casting|CastToBP_Drink OtherActor))
  (Rendering|SetVisibility (Variables|Default|GetWidget) true false)
  (Variables|/Game/Blueprints/Player/FirstPerson/BP_FirstPersonCharacter.BP_FirstPersonCharacter_C|SetcanInteract (Variables|Default|GetPlayer) true))

(event OnTargetPerceptionUpdated(AIPerception)
  (params (Actor :type Actor%20Object%20Reference) (Stimulus :type AI%20Stimulus%20Structure))
  (Utilities|Casting|CastToPlayerController Actor)
  (if (.bsuccessfullysensed Stimulus)
    (Variables|Default|SetisSeeingPlayer true)
    (else
      (Variables|Default|SetisSeeingPlayer false))))

(event OnComponentBeginOverlap(CapsuleComponent)
  (params (OverlappedComponent :type Primitive%20Component%20Object%20Reference) (OtherActor :type Actor%20Object%20Reference) (OtherComp :type Primitive%20Component%20Object%20Reference) (OtherBodyIndex :type Integer) (bFromSweep :type Boolean) (SweepResult :type Hit%20Result%20Structure%20%28by%20ref%29))
  (Utilities|Casting|CastToBP_FirstPersonCharacter OtherActor)
  (if (Variables|Default|GetisAngry)
    (Game|Damage|ApplyDamage (Variables|Default|GetPlayer) (Math|Conversions|ToFloat(Integer) (Variables|Default|GetattackDamage)) 0 0)
    (Utilities|FlowControl|Delay 2.0)))

(event OnComponentEndOverlap(RecieveDrinkCollision)
  (params (OverlappedComponent :type Primitive%20Component%20Object%20Reference) (OtherActor :type Actor%20Object%20Reference) (OtherComp :type Primitive%20Component%20Object%20Reference) (OtherBodyIndex :type Integer))
  (Rendering|SetVisibility (Variables|Default|GetWidget) false false)
  (Variables|/Game/Blueprints/Player/FirstPerson/BP_FirstPersonCharacter.BP_FirstPersonCharacter_C|SetcanInteract (Variables|Default|GetPlayer) false))

(event Custom|ActivateAngry
  (Variables|Default|SetisAngry true))

(event Custom|UseDoor
  ;[1 1 1] finds the closest place to open the door from and moves to it
  (bind _returnvalue (Actor|GetActorOfClass "/Game/Blueprints/Environment/BP_Doors.BP_Doors_C"))
  (if (Variables|Default|GetisInside)
    (AI|AIMoveTo self (Transformation|GetWorldLocation (Variables|/Game/Blueprints/Environment/BP_Doors.BP_Doors_C|GetInsideRef _returnvalue)) 0 0.5 false
      (:OnSuccess
        ;[1 1 1] Walks through the door
        (Utilities|FlowControl|Delay 1.0)
        (AI|AIMoveTo self (Transformation|GetWorldLocation (Variables|/Game/Blueprints/Environment/BP_Doors.BP_Doors_C|GetOutsideRef _returnvalue)) 0 0.5 false
          (:OnSuccess
            (Variables|Default|SetisInside false)))))
    (else
      (AI|AIMoveTo self (Transformation|GetWorldLocation (Variables|/Game/Blueprints/Environment/BP_Doors.BP_Doors_C|GetOutsideRef _returnvalue)) 0 0.5 false
        (:OnSuccess
          (Utilities|FlowControl|Delay 1.0)
          (AI|AIMoveTo self (Transformation|GetWorldLocation (Variables|/Game/Blueprints/Environment/BP_Doors.BP_Doors_C|GetInsideRef _returnvalue)) 0 0.5 false
            (:OnSuccess
              (Variables|Default|SetisInside true)
              (CallFunction|Queue))))))))

(event Custom|Queue
  ;[1 1 1] Customer goes to queue
  (bind _returnvalue (Actor|GetActorOfClass "/Game/Blueprints/Environment/BP_Bar.BP_Bar_C"))
  (AI|AIMoveTo self (Transformation|GetWorldLocation (Variables|/Game/Blueprints/Environment/BP_Bar.BP_Bar_C|GetQueuePlace0Ref _returnvalue)) 0 1.0 false
    (:OnSuccess
      (Transformation|SetActorRotation (Math|Conversions|RotationFromXVector (Math|Vector|GetForwardVector (Variables|/Game/Blueprints/Environment/BP_Bar.BP_Bar_C|GetQueuePlace0Ref _returnvalue))))
      (CallFunction|OrderDrink)
      (CallFunction|AngryTimer))))

(event Custom|OrderDrink
  (bind _outrownames (DataTable|GetDataTableRowNames "/Game/Blueprints/Drinks/DT_DrinkData.DT_DrinkData"))
  (Variables|Default|SetdrinkOrdered (.OutItem (Utilities|Array|Random _outrownames)))
  (Rendering|SetVisibility (Variables|Default|GetOrderWidget) true false))

(event Custom|AngryTimer
  (bind _returnvalue (Utilities|Time|SetTimerbyEvent (delegate Custom|ActivateAngry) (Variables|Default|GetangerActivateTime))))

(event Custom|Leave%20Pub
  (CallFunction|UseDoor)
  (bind _returnvalue (Actor|GetActorOfClass "/Game/Blueprints/Environment/BP_DespawnRef.BP_DespawnRef_C"))
  (AI|AIMoveTo self (Transformation|GetWorldLocation (Variables|/Script/Engine.Actor|GetRootComponent _returnvalue)) 0 0.5 false
    (:OnSuccess
      (Actor|DestroyActor))))

(event EventBeginPlay
  ;[1 1 1] walk into the pub when spawned in
  (bind _returnvalue (Actor|GetActorOfClass "/Game/Blueprints/Player/FirstPerson/BP_FirstPersonCharacter.BP_FirstPersonCharacter_C"))
  (Variables|Default|SetPlayer _returnvalue)
  (bind _aswb_drink_order (Utilities|Casting|CastToWB_DrinkOrder (UserInterface|GetWidget (Variables|Default|GetOrderWidget))))
  (Variables|/Game/UI/WB_DrinkOrder.WB_DrinkOrder_C|SetOwnerBP _aswb_drink_order self)
  (Variables|Default|SethappinessScoreBase (Variables|Default|GethappinessScore))
  (CallFunction|UseDoor))

(event EventInteract
  (bind _drinkordered (Variables|Default|GetdrinkOrdered))
  ;[1 1 1] If the drink the player gives is the same as the one ordered give £100+happiness score and leaves
  (if (== _drinkordered (Variables|/Game/Blueprints/Drinks/BP_Drink.BP_Drink_C|GetdrinkName (stale OnComponentBeginOverlap(RecieveDrinkCollision) _asbp_drink)))
    (Default|GiveMoneytoPlayer (Variables|Default|GetPlayer) (+ 100 (Variables|Default|GethappinessScore)))
    (CallFunction|LeavePub)
    (else
      ;[1 1 1] If the drink the player gives is the same type as the one ordered give £50+happiness score and leaves else attack the player
      (bind _returnvalue (Utilities|GetDataTableRow "/Game/Blueprints/Drinks/DT_DrinkData.DT_DrinkData" _drinkordered)
        (:then
          (bind _returnvalue_2 (Utilities|GetDataTableRow "/Game/Blueprints/Drinks/DT_DrinkData.DT_DrinkData" (Variables|/Game/Blueprints/Drinks/BP_Drink.BP_Drink_C|GetdrinkName (stale OnComponentBeginOverlap(RecieveDrinkCollision) _asbp_drink)))
            (:then
              (if (Utilities|Enum|Equal(Enum) (.drinktype _returnvalue) (.drinktype _returnvalue_2))
                (Default|GiveMoneytoPlayer (Variables|Default|GetPlayer) (+ 50 (Variables|Default|GethappinessScore)))
                (CallFunction|LeavePub)
                (else
                  (Variables|Default|SetisAngry true))))))))))

(event EventTick
  (params (DeltaSeconds :type Float%20%28single-precision%29))
  (if (Variables|Default|GetisInside)
    (if (>= (Class|KismetSystemLibrary|GetTimerElapsedTimeHandle (stale Custom|AngryTimer _returnvalue)) 0.0)
      (Variables|Default|SethappinessScore (Math|Conversions|ToInteger(Byte) (- (Variables|Default|GethappinessScoreBase) (Class|KismetMathLibrary|Round64 (* (/ (Class|KismetSystemLibrary|GetTimerElapsedTimeHandle (stale Custom|AngryTimer _returnvalue)) (Variables|Default|GetangerActivateTime)) 1e+02)))))
      (else
        (Variables|Default|SethappinessScore 0)))
    (if (Variables|Default|GetisAngry)
      (AI|AIMoveTo self "0, 0, 0" (Variables|Default|GetPlayer) 8e+01 false))))

(fn ConstructionScript)