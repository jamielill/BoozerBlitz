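; BP_Shaker is a drink-mixing shaker that collects alcohol bottles and checks them for a recipe.
; When a BP_AlcoholBottle overlaps its Box, it adds the bottle to DrinksInShaker, plays a combine sound and runs IngredientComboCheck.
; The check hardcodes one combo, playing a doorbell sound when the array contains both the Jagermeister and Red Bull actors found through GetActorOfClass.
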(event OnComponentBeginOverlap(Box)
  (params (OverlappedComponent :type Primitive%20Component%20Object%20Reference) (OtherActor :type Actor%20Object%20Reference) (OtherComp :type Primitive%20Component%20Object%20Reference) (OtherBodyIndex :type Integer) (bFromSweep :type Boolean) (SweepResult :type Hit%20Result%20Structure%20%28by%20ref%29))
  (bind _asbp_alcohol_bottle (Utilities|Casting|CastToBP_AlcoholBottle OtherActor))
  (Utilities|Array|Add (Variables|Default|GetDrinksInShaker) _asbp_alcohol_bottle)
  (Audio|SpawnSoundatLocation "/Game/Audio/SFX_Shaker_Combine.SFX_Shaker_Combine" "0, 0, 0" "0, 0, 0" 1.0 1.0 0.0 0 0)
  (CallFunction|IngredientComboCheck))

(event Custom|IngredientComboCheck
  (bind _drinksinshaker (Variables|Default|GetDrinksInShaker))
  (bind _returnvalue (Actor|GetActorOfClass "/Game/Blueprints/Bottles/BP_Bottle_Jagermeister.BP_Bottle_Jagermeister_C"))
  (bind _returnvalue_2 (Actor|GetActorOfClass "/Game/Blueprints/Bottles/BP_Bottle_RedBull.BP_Bottle_RedBull_C"))
  (if (and (Utilities|Array|ContainsItem _drinksinshaker _returnvalue) (Utilities|Array|ContainsItem _drinksinshaker _returnvalue_2))
    (Audio|SpawnSoundatLocation "/Game/Audio/SFX_DoorBell.SFX_DoorBell" "0, 0, 0" "0, 0, 0" 1.0 1.0 0.0 0 0)))

(fn ConstructionScript)