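; BP_Doors is a double door that swings open automatically for customer AI (BP_CustomerAI_Base) characters.
; Box begin overlap plays timelines that yaw the first child component of BPDoorLeft and BPDoorRight outward in opposite directions.
; End overlap reverses a separate pair of timelines from the end to close them.
; An IsOpen flag gates both directions and changes only after a delay triggered from the timeline updates.
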(event OnComponentBeginOverlap(Box)
  (params (OverlappedComponent :type Primitive%20Component%20Object%20Reference) (OtherActor :type Actor%20Object%20Reference) (OtherComp :type Primitive%20Component%20Object%20Reference) (OtherBodyIndex :type Integer) (bFromSweep :type Boolean) (SweepResult :type Hit%20Result%20Structure%20%28by%20ref%29))
  ;[1 1 1] NPC interaction
  (Utilities|Casting|CastToBP_CustomerAI_Base OtherActor)
  ;[1 1 1] Open Doors
  (if (not (Variables|Default|GetIsOpen))
    (Utilities|FlowControl|Sequence
      (:then_0
        (bind _leftdooropen (Timeline|LeftDoorOpen Play)
          (:Update
            (Transformation|SetRelativeRotation (Components|GetChildComponent (Variables|Default|GetBP_Door_Left) 0) (Math|Rotator|MakeRotator 0.0 0.0 (Math|Float|Lerp 0.0 9e+01 _leftdooropen)) false false))))
      (:then_1
        (bind _rightdooropen (Timeline|RightDoorOpen Play)
          (:Update
            (Transformation|SetRelativeRotation (Components|GetChildComponent (Variables|Default|GetBP_Door_Right) 0) (Math|Rotator|MakeRotator 0.0 0.0 (Math|Float|Lerp 0.0 -9e+01 _rightdooropen)) false false)))))
    (Utilities|FlowControl|Delay 2.0)
    (Variables|Default|SetIsOpen true)))

(event OnComponentEndOverlap(Box)
  (params (OverlappedComponent :type Primitive%20Component%20Object%20Reference) (OtherActor :type Actor%20Object%20Reference) (OtherComp :type Primitive%20Component%20Object%20Reference) (OtherBodyIndex :type Integer))
  ;[1 1 1] NPC interaction
  (Utilities|Casting|CastToBP_CustomerAI_Base OtherActor)
  ;[1 1 1] Close Doors
  (if (Variables|Default|GetIsOpen)
    (Utilities|FlowControl|Sequence
      (:then_0
        (bind _leftdooropen (Timeline|Timeline ReverseFromEnd)
          (:Update
            (Transformation|SetRelativeRotation (Components|GetChildComponent (Variables|Default|GetBP_Door_Left) 0) (Math|Rotator|MakeRotator 0.0 0.0 (Math|Float|Lerp 0.0 9e+01 _leftdooropen)) false false))))
      (:then_1
        (bind _rightdooropen (Timeline|Timeline_0 ReverseFromEnd)
          (:Update
            (Transformation|SetRelativeRotation (Components|GetChildComponent (Variables|Default|GetBP_Door_Right) 0) (Math|Rotator|MakeRotator 0.0 0.0 (Math|Float|Lerp 0.0 -9e+01 _rightdooropen)) false false)))))
    (Utilities|FlowControl|Delay 2.0)
    (Variables|Default|SetIsOpen false)))

(fn ConstructionScript)