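; Cocktail shaker actor that collects alcohol bottles and spawns a mixed drink when a recipe matches.
; A bottle entering the box shows a prompt widget and enables player interaction; Interact adds that bottle to DrinksInShaker and runs IngredientComboCheck.
; Hard-coded Jagerbomb and Espresso Martini checks match against the first GetActorOfClass instance of each ingredient, then clear the array, play a sound and spawn the cocktail.
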(event OnComponentBeginOverlap(Box)
  (params (OverlappedComponent :type Primitive%20Component%20Object%20Reference) (OtherActor :type Actor%20Object%20Reference) (OtherComp :type Primitive%20Component%20Object%20Reference) (OtherBodyIndex :type Integer) (bFromSweep :type Boolean) (SweepResult :type Hit%20Result%20Structure%20%28by%20ref%29))
  (bind _asbp_alcohol_bottle (Utilities|Casting|CastToBP_AlcoholBottle OtherActor))
  (Rendering|SetVisibility (Variables|Default|GetWidget) true false)
  (Variables|/Game/Blueprints/Player/FirstPerson/BP_FirstPersonCharacter.BP_FirstPersonCharacter_C|SetcanInteract (Variables|Default|GetPlayer) true))

(event OnComponentEndOverlap(Box)
  (params (OverlappedComponent :type Primitive%20Component%20Object%20Reference) (OtherActor :type Actor%20Object%20Reference) (OtherComp :type Primitive%20Component%20Object%20Reference) (OtherBodyIndex :type Integer))
  (Rendering|SetVisibility (Variables|Default|GetWidget) false false)
  (Variables|/Game/Blueprints/Player/FirstPerson/BP_FirstPersonCharacter.BP_FirstPersonCharacter_C|SetcanInteract (Variables|Default|GetPlayer) false))

(event Custom|IngredientComboCheck
  (bind _drinksinshaker (Variables|Default|GetDrinksInShaker))
  (bind _drinksinshaker_2 (Variables|Default|GetDrinksInShaker))
  (if (> (Utilities|Array|Length (Variables|Default|GetDrinksInShaker)) 1)
    (Utilities|FlowControl|Sequence
      (:then_0
        ;[1 1 1] Jagerbomb check
        (Utilities|FlowControl|Sequence
          (:then_0
            (bind _returnvalue (Actor|GetActorOfClass "/Game/Blueprints/Bottles/BP_Bottle_Jagermeister.BP_Bottle_Jagermeister_C")))
          (:then_1
            (bind _returnvalue_2 (Actor|GetActorOfClass "/Game/Blueprints/Bottles/BP_Bottle_RedBull.BP_Bottle_RedBull_C")))
          (:then_2
            (if (and (Utilities|Array|ContainsItem _drinksinshaker_2 _returnvalue) (Utilities|Array|ContainsItem _drinksinshaker_2 _returnvalue_2))
              (Utilities|Array|Clear (Variables|Default|GetDrinksInShaker))
              (Audio|SpawnSoundatLocation "/Game/Audio/SFX_Cocktail_Shaker.SFX_Cocktail_Shaker" "0, 0, 0" "0, 0, 0" 1.0 1.0 0.0 0 0)
              (Game|SpawnActorfromClass "/Game/Blueprints/Drinks/BP_Cocktail_JagerBomb.BP_Cocktail_JagerBomb_C" (Transformation|GetActorTransform) "Undefined" "MultiplyWithRoot" 0 0)))))
      (:then_1
        ;[1 1 1] Espresso Martini check
        (Utilities|FlowControl|Sequence
          (:then_0
            (bind _returnvalue_3 (Actor|GetActorOfClass "/Game/Blueprints/Bottles/BP_Bottle_Smirnoff.BP_Bottle_Smirnoff_C")))
          (:then_1
            (bind _returnvalue_4 (Actor|GetActorOfClass "/Game/Blueprints/Bottles/BP_Bottle_Kahlua.BP_Bottle_Kahlua_C")))
          (:then_2
            (if (and (Utilities|Array|ContainsItem _drinksinshaker _returnvalue_3) (Utilities|Array|ContainsItem _drinksinshaker _returnvalue_4))
              (Utilities|Array|Clear (Variables|Default|GetDrinksInShaker))
              (Audio|SpawnSoundatLocation "/Game/Audio/SFX_Cocktail_Shaker.SFX_Cocktail_Shaker" "0, 0, 0" "0, 0, 0" 1.0 1.0 0.0 0 0)
              (Game|SpawnActorfromClass "/Game/Blueprints/Drinks/BP_Cocktail_EspressoMartini.BP_Cocktail_EspressoMartini_C" (Transformation|GetActorTransform) "Undefined" "MultiplyWithRoot" 0 0))))))))

(event EventBeginPlay
  (bind _returnvalue (Actor|GetActorOfClass "/Game/Blueprints/Player/FirstPerson/BP_FirstPersonCharacter.BP_FirstPersonCharacter_C"))
  (Variables|Default|SetPlayer _returnvalue))

(event EventInteract
  (Utilities|Array|Add (Variables|Default|GetDrinksInShaker) (stale OnComponentBeginOverlap(Box) _asbp_alcohol_bottle))
  (Variables|/Game/Blueprints/Player/FirstPerson/BP_FirstPersonCharacter.BP_FirstPersonCharacter_C|SetcanInteract (Variables|Default|GetPlayer) false)
  (Audio|SpawnSoundatLocation "/Game/Audio/SFX_Shaker_Combine.SFX_Shaker_Combine" "0, 0, 0" "0, 0, 0" 1.0 1.0 0.0 0 0)
  (CallFunction|IngredientComboCheck))

(fn ConstructionScript)